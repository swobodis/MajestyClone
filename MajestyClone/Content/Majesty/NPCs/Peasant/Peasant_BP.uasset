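; Peasant NPC Blueprint that gives each peasant a profile and provides a build-or-repair work step.
; Construction fills the profile with character type, home reference and a name formed from the type plus the current peasant count.
; BuildorRepair, when overlapping the build job's capsule, uses ApplyDamage's return value to raise its health, clamped to max, and reports completion.
; The repair job only gets a validity check in a stopgap fallback.
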(fn ConstructionScript
  (|CallParentFunction)
  (CallFunction|SetNPCProfile0))

(fn SetNPCProfile0
  (bind _name (CallFunction|GetPeasantName))
  (Variables|Default|SetNPCProfile (Utilities|Struct|MakeNPCProfile_Struct "NewEnumerator0" _name (Variables|Default|GetHomeRef))))

(fn GetPeasantName
  (bind _outactors (Actor|GetAllActorsOfClass "Peasant_BP_C"))
  (return (Utilities|String|StringToName (Utilities|String|Append (Utilities|String|EnumtoString (Utilities|Enum|LiteralenumCharacterType_ENUM "NewEnumerator0")) (Utilities|String|ToString(Integer) (Utilities|Array|Length _outactors))))))

(fn BuildorRepair
  (bind _currentbuildjob (Variables|Default|GetCurrentBuildJob))
  (bind _currentbuildjob_2 (Variables|Default|GetCurrentBuildJob))
  (bind _currentbuildjob_3 (Variables|Default|GetCurrentBuildJob))
  (bind _currentbuildjob_4 (Variables|Default|GetCurrentBuildJob))
  (bind _maxhealth (Variables|/Game/Majesty/Buildings/Construction/ConstructionProxy_BP.ConstructionProxy_BP_C|GetMaxHealth _currentbuildjob_4))
  (if (and (Utilities|IsValid _currentbuildjob) (Collision|IsOverlappingActor (Variables|/Game/Majesty/Buildings/Construction/ConstructionProxy_BP.ConstructionProxy_BP_C|GetCapsule _currentbuildjob) self :!class /Script/Engine.PrimitiveComponent))
    (bind _returnvalue (Game|Damage|ApplyDamage _currentbuildjob_2 (Math|Conversions|ToFloat(Integer) (Variables|Default|GetAttackDamage)) 0 self))
    (bind _output_get (Variables|/Game/Majesty/Buildings/Construction/ConstructionProxy_BP.ConstructionProxy_BP_C|SetCurrentHealth (Variables|Default|GetCurrentBuildJob) (Math|Integer|Clamp(Integer) (+ (Variables|/Game/Majesty/Buildings/Construction/ConstructionProxy_BP.ConstructionProxy_BP_C|GetCurrentHealth _currentbuildjob_2) (Math|Float|Truncate _returnvalue)) 0 _maxhealth)))
    (Development|PrintString (Utilities|String|ToString(Integer) _output_get) true true "(R=0.000000,G=0.660000,B=1.000000,A=1.000000)" 5.0)
    (return (== _maxhealth (Variables|/Game/Majesty/Buildings/Construction/ConstructionProxy_BP.ConstructionProxy_BP_C|GetCurrentHealth _currentbuildjob_4)))
    (elif (not (Utilities|IsValid (Variables|Default|GetCurrentRepairJob)))
      ;[1 1 1] not the right way to handle this
      (return (== (Variables|/Game/Majesty/Buildings/Construction/ConstructionProxy_BP.ConstructionProxy_BP_C|GetMaxHealth _currentbuildjob_3) (Variables|/Game/Majesty/Buildings/Construction/ConstructionProxy_BP.ConstructionProxy_BP_C|GetCurrentHealth _currentbuildjob_3))))))