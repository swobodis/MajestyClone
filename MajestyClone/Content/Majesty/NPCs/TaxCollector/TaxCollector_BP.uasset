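; Tax collector NPC that carries gold from collection job buildings back to its home.
; Construction fills its NPC profile with a character type, its home reference and a name built from the type plus the current collector count.
; CollectGold empties the current job's stored gold into the carried total and clears the job.
; DepositGold hides the collector, disables its collision and banks the gold at HomeRef, with the Palace check left unwired.
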(event EventBeginPlay
  (|CallParentFunction))

(event Game|Damage|EventAnyDamage
  (params (Damage :type Float%20%28single-precision%29) (DamageType :type Damage%20Type%20Object%20Reference) (InstigatedBy :type Controller%20Object%20Reference) (DamageCauser :type Actor%20Object%20Reference))
  (CallFunction|TakeDamage Damage))

(fn ConstructionScript
  (|CallParentFunction)
  (bind _name (CallFunction|GetTaxCollectorName))
  (Variables|Default|SetNPCProfile (Utilities|Struct|MakeNPCProfile_Struct "NewEnumerator2" _name (Variables|Default|GetHomeRef))))

(fn GetTaxCollectorName
  (bind _outactors (Actor|GetAllActorsOfClass "TaxCollector_BP_C"))
  (return (Utilities|String|StringToName (Utilities|String|Append (Utilities|String|EnumtoString (Utilities|Enum|LiteralenumCharacterType_ENUM "NewEnumerator2")) (Utilities|String|ToString(Integer) (Utilities|Array|Length _outactors))))))

(fn DepositGold
  (bind _homeref (Variables|Default|GetHomeRef))
  (Rendering|SetActorHiddenInGame true)
  (Collision|SetActorEnableCollision false)
  (if true
    (Variables|/Game/Majesty/Buildings/BuildingMasterBP.BuildingMasterBP_C|SetGoldStored _homeref (+ (Variables|Default|GetGoldCarried) (Variables|/Game/Majesty/Buildings/BuildingMasterBP.BuildingMasterBP_C|GetGoldStored _homeref)))
    (Variables|Default|SetGoldCarried 0)
    (return)
    (else
      (Development|PrintString "Palace is not HomeRef")
      (return))))

(fn CollectGold
  (bind _output_get (Variables|Default|SetGoldCarried (+ (Variables|/Game/Majesty/Buildings/BuildingMasterBP.BuildingMasterBP_C|GetGoldStored (Variables|Default|GetCurrentCollectionJob)) (Variables|Default|GetGoldCarried))))
  (Development|PrintString (Utilities|String|ToString(Integer) _output_get))
  (Variables|/Game/Majesty/Buildings/BuildingMasterBP.BuildingMasterBP_C|SetGoldStored (Variables|Default|GetCurrentCollectionJob) 0)
  (Variables|Default|SetCurrentCollectionJob 0)
  (return))