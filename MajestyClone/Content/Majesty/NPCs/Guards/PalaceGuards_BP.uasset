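; Palace guard NPC actor that takes damage and dies when its health runs out.
; Any damage lowers its current health, updates the progress bar in its Healthbar widget component to the remaining fraction, and prints the value as debug text.
; The actor is destroyed at zero health or below, a check that is skipped if the widget cast fails.
; BeginPlay and construction only call the parent class.
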(event Game|Damage|EventAnyDamage
  (params (Damage :type Float%20%28single-precision%29) (DamageType :type Damage%20Type%20Object%20Reference) (InstigatedBy :type Controller%20Object%20Reference) (DamageCauser :type Actor%20Object%20Reference))
  (Variables|Default|SetCurrentHealth (- (Variables|Default|GetCurrentHealth) Damage))
  (bind _ashealthbar (Utilities|Casting|CastToHealthbar (UserInterface|GetUserWidgetObject (Variables|Default|GetWidget))))
  (Progress|SetPercent (Variables|/Game/Majesty/NPCs/Healthbar.Healthbar_C|GetHealthbar _ashealthbar) (/ (Variables|Default|GetCurrentHealth) (Variables|Default|GetMaxHealth)))
  (Development|PrintString (Utilities|String|ToString(Float) (Variables|Default|GetCurrentHealth)) true true "(R=1.000000,G=0.031642,B=0.221980,A=1.000000)")
  (if (<= (Variables|Default|GetCurrentHealth) 0.0)
    (Actor|DestroyActor)))

(event EventBeginPlay
  (|CallParentFunction))

(fn ConstructionScript
  (|CallParentFunction))