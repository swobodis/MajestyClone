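; Tax collector NPC Blueprint that sets up its own identity profile on top of its parent class's construction.
; The construction script fills NPCProfile with a character type, a generated name and its home reference.
; GetTaxCollectorName builds that name by appending the current count of TaxCollector_BP actors in the level to the character type's enum string.
; The event graph holds no active logic.
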(event EventBeginPlay)

(fn ConstructionScript
  (|CallParentFunction)
  (bind _name (CallFunction|GetTaxCollectorName))
  (Variables|Default|SetNPCProfile (Utilities|Struct|MakeNPCProfile_Struct "NewEnumerator2" _name (Variables|Default|GetHomeRef))))

(fn GetTaxCollectorName
  (bind _outactors (Actor|GetAllActorsOfClass "TaxCollector_BP_C"))
  (return (Utilities|String|StringToName (Utilities|String|Append (Utilities|String|EnumtoString (Utilities|Enum|LiteralenumCharacterType_ENUM "NewEnumerator2")) (Utilities|String|ToString(Integer) (Utilities|Array|Length _outactors))))))