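; Palace building that keeps its staff of peasants, tax collectors and palace guards topped up.
; A looping timer spawns units at the entrance sphere, with guards after a short delay, and sets the palace as their home.
; Check functions return each type's maximum minus its world-wide count.
; Peasants and guards require pending ConstructionManager proxies, while tax collectors require a non-empty game state collection queue.
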(event Custom|RunSequence
  (bind _entrancesphere (Variables|Default|GetEntranceSphere))
  (bind _entrancesphere_2 (Variables|Default|GetEntranceSphere))
  (bind _returnvalue (Transformation|GetWorldTransform _entrancesphere))
  (bind _returnvalue_2 (Transformation|GetWorldTransform _entrancesphere_2))
  (Utilities|FlowControl|Sequence
    (:then_0
      ;[1 1 1] Spawn Peasant
      (bind _peasantsneeded (CallFunction|CheckPeasants))
      (for _index (range 1 _peasantsneeded)
        (bind _returnvalue_3 (Game|SpawnActorfromClass "/Game/Majesty/NPCs/Peasant/Peasant_BP.Peasant_BP_C" (Math|Transform|MakeTransform (Math|Vector|MakeVector (.x (.location _returnvalue_2)) (.y (.location _returnvalue_2)) 6e+01) (.rotation _returnvalue_2) "0.500000,0.500000,0.500000") "AdjustIfPossibleButAlwaysSpawn" 0 0))
        (Variables|/Game/Majesty/NPCs/NPCMaster_BP.NPCMaster_BP_C|SetHomeRef _returnvalue_3 self)))
    (:then_1
      ;[1 1 1] Spawn Tax Collector
      (bind _taxcollectorsneeded (CallFunction|CheckTaxCollectors))
      (for _index_2 (range 1 _taxcollectorsneeded)
        (bind _returnvalue_4 (Game|SpawnActorfromClass "/Game/Majesty/NPCs/TaxCollector/TaxCollector_BP.TaxCollector_BP_C" (Math|Transform|MakeTransform (Math|Vector|MakeVector (.x (.location _returnvalue)) (.y (.location _returnvalue)) 6e+01) (.rotation _returnvalue) "0.500000,0.500000,0.500000") "AdjustIfPossibleButAlwaysSpawn" 0 0))
        (Variables|/Game/Majesty/NPCs/NPCMaster_BP.NPCMaster_BP_C|SetHomeRef _returnvalue_4 self)))
    (:then_2
      ;[1 1 1] Spawn Guards
      (Utilities|FlowControl|Delay 2.0)
      (bind _guardsneeded (CallFunction|CheckGuards))
      (for _index_3 (range 1 _guardsneeded)
        (bind _returnvalue_5 (Game|SpawnActorfromClass "/Game/Majesty/NPCs/Guards/PalaceGuards_BP.PalaceGuards_BP_C" (Math|Transform|MakeTransform (Math|Vector|MakeVector (.x (.location _returnvalue)) (.y (.location _returnvalue)) 6e+01) (.rotation _returnvalue) "0.500000,0.500000,0.500000") "AdjustIfPossibleButAlwaysSpawn" 0 0))
        (Variables|/Game/Majesty/NPCs/NPCMaster_BP.NPCMaster_BP_C|SetHomeRef _returnvalue_5 self)))))

(event EventBeginPlay
  (Utilities|Time|SetTimerbyEvent (delegate Custom|RunSequence) 5.0 true)
  (bind _asmain_camera_controller (Utilities|Casting|CastToMainCameraController (Game|GetPlayerController 0)))
  (Variables|References|SetConstructionManager (Variables|/Game/Majesty/GameBP/MainCameraController.MainCameraController_C|GetConstructionManagerRef _asmain_camera_controller)))

(fn ConstructionScript
  (|CallParentFunction))

(fn CheckPeasants
  (if (> (Utilities|Array|Length (Variables|/Game/Majesty/Buildings/Construction/ConstructionManager_BP.ConstructionManager_BP_C|GetProxies (Variables|References|GetConstructionManager))) 0)
    (bind _outactors (Actor|GetAllActorsOfClass "/Game/Majesty/NPCs/Peasant/Peasant_BP.Peasant_BP_C"))
    (return (- (Variables|Default|GetMaxPeasants) (Utilities|Array|Length _outactors)))
    (else
      (return 0))))

(fn CheckGuards
  (if (> (Utilities|Array|Length (Variables|/Game/Majesty/Buildings/Construction/ConstructionManager_BP.ConstructionManager_BP_C|GetProxies (Variables|References|GetConstructionManager))) 0)
    (bind _outactors (Actor|GetAllActorsOfClass "/Game/Majesty/NPCs/Guards/PalaceGuards_BP.PalaceGuards_BP_C"))
    (return (- (Variables|Default|GetMaxGuards) (Utilities|Array|Length _outactors)))
    (else
      (return 0))))

(fn CheckTaxCollectors
  (if (> (Utilities|Array|Length (Variables|/Game/Majesty/GameBP/MajestyGameState.MajestyGameState_C|GetCollectionQueue (.AsMajesty%20Game%20State (Utilities|Casting|CastToMajestyGameState (Game|GetGameState))))) 0)
    (bind _outactors (Actor|GetAllActorsOfClass "/Game/Majesty/NPCs/TaxCollector/TaxCollector_BP.TaxCollector_BP_C"))
    (return (- (Variables|Default|GetMaxTaxCollectors) (Utilities|Array|Length _outactors)))
    (else
      (return 0))))