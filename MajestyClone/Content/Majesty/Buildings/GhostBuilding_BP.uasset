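; Ghost building actor that shows a building's display mesh, likely as a construction preview.
; OnSpawn stores the mesh and class and sets the static mesh only while inactive; KillGhost clears that state but leaves the component's mesh in place.
; ConstructBuilding spawns the given building at world origin with a controller reference, then, if the cast succeeds, resets the ghost and reactivates it with that building's mesh.
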(event Custom|OnSpawn
  (params (DisplayMesh :type Static%20Mesh%20Object%20Reference) (BuildingClass :type Building%20Master%20BP%20Class%20Reference))
  ;[1 1 1] OnSpawn
  (if (not (Variables|Default|GetIsActive))
    (Variables|Default|SetBuildingClass BuildingClass)
    (Variables|Default|SetDisplayMesh DisplayMesh)
    (Variables|Default|SetIsActive true)
    (Components|StaticMesh|SetStaticMesh (Variables|Default|GetGhostBuilding_Mesh) (Variables|Default|GetDisplayMesh))))

(event Custom|KillGhost
  ;[1 1 1] Kill Ghost
  (Variables|Default|SetBuildingClass 0)
  (Variables|Default|SetDisplayMesh 0)
  (Variables|Default|SetIsActive false))

(event EventConstructBuilding
  (params (MainBuilding :type Building%20Master%20BP%20Class%20Reference))
  ;[1 1 1] Event Construct Building
  (bind _returnvalue (Game|SpawnActorfromClass MainBuilding (Math|Transform|MakeTransform "0, 0, 0") "Undefined" 0 (Variables|Default|GetControllerRef) 0))
  (bind _asbuilding_master_bp (Utilities|Casting|CastToBuildingMasterBPClass MainBuilding))
  (CallFunction|KillGhost)
  (CallFunction|OnSpawn (Variables|/Game/Majesty/Buildings/BuildingMasterBP.BuildingMasterBP_C|GetDisplayMesh _returnvalue) _asbuilding_master_bp))

(fn ConstructionScript)