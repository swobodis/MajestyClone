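; Construction proxy Blueprint that stands in for a building under construction, shown as a ghost of its display mesh.
; The construction script assigns DisplayMesh with the Ghost_M_Inst material on its first slot, then calls SetCapsuleArea with the capsule and mesh.
; Tick fires ConstructionCompleted on every frame that IsConstructionCompleted is true.
; SetMaxBuildingHealth stores the building's maximum health.
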(event EventTick
  (params (DeltaSeconds :type Float%20%28single-precision%29))
  (if (Variables|Default|GetIsConstructionCompleted)
    (Default|CallConstructionCompleted self)))

(fn ConstructionScript
  (Components|StaticMesh|SetStaticMesh (Variables|Default|GetStaticMesh) (Variables|Default|GetDisplayMesh))
  (Rendering|Material|SetMaterial (Variables|Default|GetStaticMesh) 0 "/Game/Majesty/Materials/Ghost_M_Inst.Ghost_M_Inst")
  (CallFunction|SetCapsuleArea (Variables|Default|GetCapsule) (Variables|Default|GetStaticMesh)))

(fn SetMaxBuildingHealth
  (params (BuildingHealth :type Integer))
  (Variables|Default|SetMaxHealth BuildingHealth)
  (return))