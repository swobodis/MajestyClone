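; BuildingMasterBP is a building actor, apparently the base for Majesty's buildings, with mesh, health and selection HUD display.
; Its construction script applies the display mesh, offsets an entrance sphere using the mesh bounds, sets the capsule area and fills health to maximum.
; BeginPlay caches the main camera controller.
; DisplayHUD creates a selected-building widget and, if the hit actor is itself, swaps it into the HUD overlay; the controller binding is disconnected.
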(event Custom|DisplayHUD
  (params (HitActor :type Actor%20Object%20Reference) (MainHudReference :type UI%20Main%20Hud%20Object%20Reference))
  (bind _mainmenuoverlay (Variables|/Game/Majesty/Huds/UI_MainHud.UI_MainHud_C|GetMainMenuOverlay MainHudReference))
  ;[1 1 1] DisplayHUD
  (bind _returnvalue (UserInterface|CreateWidget "/Game/Majesty/Huds/UI_SelectedBuilding.UI_SelectedBuilding_C" 0 HitActor))
  (Default|GetSelectedBuildingData _returnvalue)
  (Variables|References|SetSelectedBuildingHUDRef _returnvalue)
  (if (== HitActor self)
    (if (Class|PanelWidget|HasAnyChildren _mainmenuoverlay)
      (Widget|Panel|ClearChildren _mainmenuoverlay))
    (Class|Overlay|AddChildtoOverlay _mainmenuoverlay (Variables|References|GetSelectedBuildingHUDRef))))

(event EventBeginPlay
  (bind _asmain_camera_controller (Utilities|Casting|CastToMainCameraController (Game|GetPlayerController 0))
    (:then
      (Variables|References|SetControllerRef _asmain_camera_controller)
      (Development|PrintString "set worked"))
    (:CastFailed
      (Development|PrintString "set failed"))))

(fn ConstructionScript
  (Components|StaticMesh|SetStaticMesh (Variables|Default|GetStaticMesh) (Variables|BuildingInfo|GetDisplayMesh))
  (CallFunction|SetBuildingEntrance (Variables|Default|GetEntranceSphere) (Variables|Default|GetStaticMesh))
  (CallFunction|SetCapsuleArea (Variables|Default|GetCapsule) (Variables|Default|GetStaticMesh))
  (Variables|BuildingInfo|SetCurrentBuildingHealth (Variables|BuildingInfo|GetMaxBuildingHealth)))

(fn SetBuildingEntrance
  (params (Entrance :type Static%20Mesh%20Component%20Object%20Reference) (BuildingMesh :type Static%20Mesh%20Component%20Object%20Reference))
  (Transformation|SetRelativeLocation Entrance (Math|Vector|MakeVector 0.0 (+ (Math|Float|Absolute(Float) (.y (.Min (Components|StaticMesh|GetLocalBounds BuildingMesh)))) (LocalVariables|GetEntranceDistance)) 32.0) false false))