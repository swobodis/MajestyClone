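; Rangers Guild building that recruits Ranger units in exchange for treasury gold.
; RecruitRanger checks the GameState treasury against the recruitment cost, then withdraws it and spawns a Ranger_BP at the EntranceSphere transform.
; Each new ranger stores this guild as its HomeRef, and insufficient funds only print a message.
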(event Custom|RecruitRanger
  (bind _recruitmentcost (Variables|Default|GetRecruitmentCost))
  (if (>= (Variables|/Game/Majesty/GameBP/MajestyGameState.MajestyGameState_C|GetTreasury (Variables|Default|GetGameStateRef)) _recruitmentcost)
    (Default|ProcessWithdrawal (Variables|Default|GetGameStateRef) _recruitmentcost)
    (bind _returnvalue (Game|SpawnActorfromClass "/Game/Majesty/NPCs/Heroes/Rangers/Ranger_BP.Ranger_BP_C" (Transformation|GetWorldTransform (Variables|Default|GetEntranceSphere)) "Undefined" 0 0))
    (Variables|/Game/Majesty/NPCs/NPCMaster_BP.NPCMaster_BP_C|SetHomeRef _returnvalue self)
    (else
      (Development|PrintString "Insufficient Funds"))))

(event EventBeginPlay
  (|CallParentFunction))

(fn ConstructionScript
  (|CallParentFunction))